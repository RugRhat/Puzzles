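; Game mode for a puzzle game that handles where BP_PuzzleSolver players spawn and respawn.
; New players alternate between starts "PS 1" and "PS 2" through a FlipFlop.
; BeginPlay records "PS 3" as the most recent start on every existing solver.
; PlayerFell destroys the fallen pawn and restarts its controller at that pawn's stored MostRecentPlayerStart.
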(event `self.ReceiveBeginPlay`
  (bind _outactors (`GameplayStatics.GetAllActorsOfClass` "/Game/Blueprints/BP_PuzzleSolver.BP_PuzzleSolver_C"))
  (for _array_element _outactors
    (bind _asplayer_start (cast `PlayerStart` (`self.K2_FindPlayerStart` (`Pawn.GetController` _array_element) "PS 3")))
    (set `/Game/Blueprints/BP_PuzzleSolver.Most Recent Player Start` _asplayer_start _array_element)))

(event `Player Fell`
  (params (`Player That Fell` :type "/Game/Blueprints/BP_PuzzleSolver Object Reference"))
  (bind _output_get (set `self.Player Controller` (`Pawn.GetController` `Player That Fell`)))
  (bind _output_get_2 (set `self.Start Spot` (`/Game/Blueprints/BP_PuzzleSolver.Most Recent Player Start` `Player That Fell`)))
  (`self.K2_DestroyActor` `Player That Fell`)
  (`self.RestartPlayerAtPlayerStart` _output_get _output_get_2))

(event `self.HandleStartingNewPlayer`
  (params (NewPlayer :type "PlayerController Object Reference"))
  (`/Engine/EditorBlueprintResources/StandardMacros.FlipFlop`
    (:`A`
      (`self.RestartPlayerAtPlayerStart` NewPlayer (`self.K2_FindPlayerStart` NewPlayer "PS 1")))
    (:`B`
      (`self.RestartPlayerAtPlayerStart` NewPlayer (`self.K2_FindPlayerStart` NewPlayer "PS 2")))))

(fn `UserConstructionScript`)